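; Spawner actor that scatters BP_Spark2 actors at random spots within its Bound component's bounds, in batches of SpawnAmount.
; BeginPlay spawns the first batch, then after a delay sets a looping timer that repeats it.
; SpawnElectro line-traces WorldStatic objects from a raised random point and spawns an enlarged spark at any blocking hit.
; The trace end adds 100000 to the negated up vector instead of scaling it, so it is not straight down.
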(event Custom|SpawnElectroAgain
  (for _index (range 1 (Variables|Default|GetSpawnAmount))
    (CallFunction|SpawnElectro)))

(event EventBeginPlay
  (for _index (range 1 (Variables|Default|GetSpawnAmount))
    (CallFunction|SpawnElectro)
    (Utilities|FlowControl|Delay 5.0)
    (Utilities|Time|SetTimerbyEvent (delegate Custom|SpawnElectroAgain) 5.0 true)))

(fn ConstructionScript)

(fn SpawnElectro
  (bind _bound (Variables|Default|GetBound))
  (bind (_origin _boxextent) (Collision|GetComponentBounds _bound))
  (bind _returnvalue (Math|Random|RandomPointinBoundingBox _origin _boxextent))
  (bind (_x _y _z) (Math|Vector|BreakVector _returnvalue))
  (bind _returnvalue_2 (+ _z 1e+03))
  (bind _returnvalue_3 (Math|Vector|MakeVector _x _y _returnvalue_2))
  (bind _outhit (Collision|LineTraceForObjects _returnvalue_3 (+ _returnvalue_3 (+ (* (Transformation|GetActorUpVector) -1) 1e+05)) (Utilities|Array|MakeArray "ObjectTypeQuery1") false 0 "None"))
  (if (.bBlockingHit (Collision|BreakHitResult _outhit))
    (Game|SpawnActorfromClass "/Game/OurContent/BP_Spark2.BP_Spark2_C" (Math|Transform|MakeTransform (.ImpactPoint (Collision|BreakHitResult _outhit)) (Math|Rotator|MakeRotator 0.0 0.0 (Math|Random|RandomFloat)) "3.000000,3.000000,3.000000") "AdjustIfPossibleButAlwaysSpawn" 0 0)))